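; Prototype player pawn that slides and rotates its origin component by mouse to kick, with keys to spawn and destroy balls.
; Mouse axes drive clamped sideways movement and free pitch, the latter locked while coiling or returning.
; Holding left click coils the pitch backward on Tick; release derives kick speed from coil angle, boosted by a delayed power flag.
; Tick then swings forward and returns toward neutral; impulse-based launch remains as disconnected backup.
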(event EventTick
  (params (DeltaSeconds :type Float%20%28single-precision%29))
  (bind _oringin (Variables|Default|GetOringin))
  (bind _oringin_2 (Variables|Default|GetOringin))
  (bind _oringin_3 (Variables|Default|GetOringin))
  (bind _relativerotation (Variables|/Script/Engine.SceneComponent|GetRelativeRotation _oringin))
  ;[0 0.4818 0.6469] Hold - Kick Coil
  (if (Variables|Default|GetHold)
    (if (> (.pitch _relativerotation) -89.0)
      (Transformation|AddLocalRotation _oringin (Math|Rotator|MakeRotator 0.0 (Math|Float|MapRangeClamped (.pitch _relativerotation) -89.0 0.0 -0.5 -2.0) 0.0) false false)
      ;[1 0.09063 0.09063] Power Kick Verification
      (if (>= (Variables|Default|GetKick%20Speed) 1e+01)
        (Utilities|FlowControl|RetriggerableDelay 0.7) ; Preciso de um Timer Melhor, que dê reset
        (if (Variables|Default|GetHold)
          (Variables|Default|SetPower%20Kick%20Loaded true)
          (Development|PrintString "Powered" true true "(R=1.000000,G=0.026667,B=0.000000,A=1.000000)"))))
    (else
      ;[1 0.3894 0] Kick Release
      (if (Variables|Default|GetRelease)
        (Variables|Default|SetMust%20Return true)
        (if (< (.pitch (Variables|/Script/Engine.SceneComponent|GetRelativeRotation _oringin_3)) (Math|Float|MapRangeClamped (Variables|Default|GetKick%20Speed) 0.0 2e+01 0.0 45.0))
          (Transformation|AddLocalRotation _oringin_3 (Math|Rotator|MakeRotator 0.0 (Variables|Default|GetKick%20Speed) 0.0) false false)
          (Variables|Default|SetMust%20Return true)
          (else
            (Variables|Default|SetRelease false)))
        (else
          ;[0.5048 1 0.4208] Return to 0
          (if (Variables|Default|GetMust%20Return)
            (Variables|Default|SetMust%20Return true)
            (if (> (.pitch (Variables|/Script/Engine.SceneComponent|GetRelativeRotation _oringin_2)) 0.0)
              (Transformation|AddLocalRotation _oringin_2 (Math|Rotator|MakeRotator 0.0 (Variables|Default|GetReturn%20Speed) 0.0) false false)
              (Utilities|FlowControl|Delay 0.3)
              (Development|PrintString "Returning" true true "(R=0.279249,G=1.000000,B=0.192994,A=1.000000)")
              (Variables|Default|SetMust%20Return false))
            (else
              (Variables|Default|SetMust%20Return false))))))))

(event Input|MouseEvents|MouseY
  (params (AxisValue :type Float%20%28single-precision%29))
  (bind _oringin (Variables|Default|GetOringin))
  (bind _relativelocation (Variables|/Script/Engine.SceneComponent|GetRelativeLocation _oringin))
  ;[0.4304 0.4119 1] Pawn Mouse Movement
  (Transformation|AddLocalOffset (Variables|Default|GetOringin) (Math|Vector|MakeVector 0.0 (* AxisValue -1e+01) 0.0) false false)
  (if (< (.y _relativelocation) -7.8e+02)
    (Transformation|SetRelativeLocation (Variables|Default|GetOringin) (Math|Vector|MakeVector 0.0 -7.8e+02 0.0) false false)
    (elif (> (.y _relativelocation) 7.8e+02)
      (Transformation|SetRelativeLocation (Variables|Default|GetOringin) (Math|Vector|MakeVector 0.0 7.8e+02 0.0) false false))))

(event Input|MouseEvents|MouseX
  (params (AxisValue :type Float%20%28single-precision%29))
  (bind _oringin (Variables|Default|GetOringin))
  (bind _relativerotation (Variables|/Script/Engine.SceneComponent|GetRelativeRotation _oringin))
  ;[1 0.4843 0.9246] Pawn Mouse Rotation
  (if (not (Variables|Default|GetHold))
    (if (not (Variables|Default|GetMust%20Return))
      (Transformation|AddLocalRotation (Variables|Default|GetOringin) (Math|Rotator|MakeRotator 0.0 (Math|Float|MapRangeClamped AxisValue -3e+01 3e+01 -1e+01 1e+01) 0.0) false false)
      (if (< (.pitch _relativerotation) -45.0)
        (Transformation|SetRelativeRotation (Variables|Default|GetOringin) (Math|Rotator|MakeRotator 0.0 -45.0 0.0) false false)
        (elif (> (.pitch _relativerotation) 45.0)
          (Transformation|SetRelativeRotation (Variables|Default|GetOringin) (Math|Rotator|MakeRotator 0.0 45.0 0.0) false false))))))

(event Input|MouseEvents|LeftMouseButton
  (params (Key :type Key%20Structure :default "None"))
  (bind _oringin (Variables|Default|GetOringin))
  (bind _relativerotation (Variables|/Script/Engine.SceneComponent|GetRelativeRotation _oringin))
  (bind _returnvalue (Math|Float|MapRangeClamped (.pitch _relativerotation) 0.0 -89.0 1.0 1e+01))
  ;[0.2219 0.2219 0.2219] Input + Hold & Release Verification
  (:Pressed
    (Variables|Default|SetHold true)
    (Variables|Default|SetRelease false)
    (Variables|Default|SetPower%20Kick%20Loaded false))
  (:Released
    (Variables|Default|SetRelease true)
    (Variables|Default|SetHold false)
    (if false
      (Variables|Default|SetPower%20Kick%20Loaded false)
      (else
        ;[1 0.8602 0.5309] Kick Speed
        (if (>= _returnvalue 1e+01)
          (if (Variables|Default|GetPower%20Kick%20Loaded)
            (bind _output_get (Variables|Default|SetKick%20Speed 2e+01))
            (Development|PrintString (Utilities|String|ToString(Float) _output_get))
            (else
              (bind _output_get_2 (Variables|Default|SetKick%20Speed 15.0))
              (Development|PrintString (Utilities|String|ToString(Float) _output_get_2))))
          (else
            (bind _output_get_3 (Variables|Default|SetKick%20Speed _returnvalue))
            (Development|PrintString (Utilities|String|ToString(Float) _output_get_3) true true "(R=0.199587,G=1.000000,B=0.000000,A=1.000000)" 5.0)))))))

(event Input|KeyboardEvents|Enter
  (params (Key :type Key%20Structure :default "None"))
  ;[1 1 1] Ball Spawn
  (:Pressed
    (bind _returnvalue (Actor|GetActorOfClass "/Game/Campo_Prototipo_Small/BP_BallSpawner.BP_BallSpawner_C"))
    (Default|SpawnBall _returnvalue)))

(event Input|KeyboardEvents|Backspace
  (params (Key :type Key%20Structure :default "None"))
  ;[0 0 0] Destroy Ball
  (:Pressed
    (bind _returnvalue (Actor|GetActorOfClass "/Game/Campo_Prototipo_Small/BP_Ball_V2.BP_Ball_V2_C"))
    (Actor|DestroyActor _returnvalue)))

(fn ConstructionScript)