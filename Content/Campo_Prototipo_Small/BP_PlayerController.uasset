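; BP_PlayerController is a prototype player controller that tells apart network roles on BeginPlay and sets up Enhanced Input.
; It branches on local controller, authority and local pawn control, printing debug labels for net client, standalone and client cases.
; Only the authoritative, locally controlled branch, labeled standalone, adds the IA_InputMapping context after a short delay.
; The net client branch only prints, so it adds no mapping context here.
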(event EventBeginPlay
  ;[0.01771 0.01771 0.01771] Distinção entre tipos de Jogador
  ;;[1 0 0] Begin Play
  ;;[1 1 1] Client Vs Server
  (if (and (Pawn|IsLocalController) (not (Ability|HasAuthority)))
    ;;[0 1 0.2018] Net Client
    (Development|PrintString "NET CLIENT")
    (else
      ;;[1 1 1] Confirmed Listen Server
      (if (Pawn|IsLocallyControlled (Pawn|GetControlledPawn))
        ;;[1 1 1] Standalone vs Client
        (if (Ability|HasAuthority)
          ;;[0 0 0] Standalone
          (Development|PrintString "STANDALONE")
          ;[0.6469 0.6469 0.6469] Mapping Context
          (Utilities|FlowControl|Delay 0.2)
          (if (Pawn|IsLocalController)
            (Input|AddMappingContext (PlayerController|LocalPlayerSubsystems|GetEnhancedInputLocalPlayerSubsystem) "/Game/Campo_Prototipo_Small/IA_InputMapping.IA_InputMapping" 0 "(bIgnoreAllPressedKeysUntilRelease=True,bForceImmediately=False,bNotifyUserSettings=False)"))
          (else
            ;;[1 0 0.9084] Client
            (Development|PrintString "Client of Listen Server")))
        (else
          ;;[0 0.1549 1] Dedicated Server & Server of the Listen Server
          (Development|PrintString "Hello" false))))))

(fn ConstructionScript)